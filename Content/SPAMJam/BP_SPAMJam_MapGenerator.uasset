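; BP_SPAMJam_MapGenerator builds a SPAMJam corridor at BeginPlay from grids of spawned actors forming a floor and two side walls.
; Nested loops space the pieces using count and spacer variables, offset from the player controller's location, with wall height in absolute Z.
; The right wall mirrors the left across Y with a 180-degree rotation.
; Spawned pieces go into FloorCubes and WallCubes arrays, and wall loops print debug positions.
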(event `self.ReceiveBeginPlay`
  (`self.Create Floor`)
  (`self.Create Left Wall`)
  (`self.CreateRightWall`))

(fn `Create Floor`
  (bind _returnvalue (`self.GetTransform` (`/Game/SPAMJam/BPL_SPAMJam.GetSPAMPlayerController`)))
  (for _index (range (+ (`self.FloorLength`) 1))
    (set `self.i` (`KismetMathLibrary.Conv_IntToDouble` _index))
    (for _index_2 (range (+ (`self.FloorWidth`) 1))
      (set `self.j` (`KismetMathLibrary.Conv_IntToDouble` _index_2))
      (bind _returnvalue_2 (`|SpawnActorFromClass` "/Game/SPAMJam/FloorPlane.FloorPlane_C" (`KismetMathLibrary.MakeTransform` (`KismetMathLibrary.MakeVector` (+ (* (`self.i`) (`self.spacer_FloorLength`)) (.x (.location _returnvalue))) (- (+ (* (`self.j`) (`self.spacer_FloorWidth`)) (.y (.location _returnvalue))) 300.0))) "Undefined" "MultiplyWithRoot" self null))
      (`KismetArrayLibrary.Array_Add` (`self.FloorCubes`) _returnvalue_2))))

(fn `Create Left Wall`
  (bind _returnvalue (`self.GetTransform` (`/Game/SPAMJam/BPL_SPAMJam.GetSPAMPlayerController`)))
  (bind _returnvalue_2 (+ (* (`self.i`) (`self.spacer_WallDistance`)) -100.0))
  (for _index (range (+ (`self.WallDistance`) 1))
    (set `self.i` (`KismetMathLibrary.Conv_IntToDouble` _index))
    (for _index_2 (range (+ (`self.WallHeight`) 1))
      (set `self.j` (`KismetMathLibrary.Conv_IntToDouble` _index_2))
      (`KismetSystemLibrary.PrintString` (`KismetStringLibrary.Conv_DoubleToString` _returnvalue_2))
      (bind _returnvalue_3 (`|SpawnActorFromClass` "/Game/SPAMJam/WallPlane.WallPlane_C" (`KismetMathLibrary.MakeTransform` (`KismetMathLibrary.MakeVector` (+ _returnvalue_2 (.x (.location _returnvalue))) (+ (.y (.location _returnvalue)) -340.0) (+ (* (`self.j`) (`self.spacer_WallHeight`)) -65.0))) "Undefined" "MultiplyWithRoot" self null))
      (`KismetArrayLibrary.Array_Add` (`self.WallCubes`) _returnvalue_3))))

(fn `CreateRightWall`
  (bind _returnvalue (`self.GetTransform` (`/Game/SPAMJam/BPL_SPAMJam.GetSPAMPlayerController`)))
  (bind _returnvalue_2 (+ (* (`self.i`) (`self.spacer_WallDistance`)) -100.0))
  (for _index (range (+ (`self.WallDistance`) 1))
    (set `self.i` (`KismetMathLibrary.Conv_IntToDouble` _index))
    (for _index_2 (range (+ (`self.WallHeight`) 1))
      (set `self.j` (`KismetMathLibrary.Conv_IntToDouble` _index_2))
      (`KismetSystemLibrary.PrintString` (`KismetStringLibrary.Conv_DoubleToString` _returnvalue_2))
      (bind _returnvalue_3 (`|SpawnActorFromClass` "/Game/SPAMJam/WallPlane.WallPlane_C" (`KismetMathLibrary.MakeTransform` (`KismetMathLibrary.MakeVector` (+ _returnvalue_2 (.x (.location _returnvalue))) (+ (.y (.location _returnvalue)) 340.0) (+ (* (`self.j`) (`self.spacer_WallHeight`)) -65.0)) (struct :`Yaw` 180.0)) "Undefined" "MultiplyWithRoot" self null))
      (`KismetArrayLibrary.Array_Add` (`self.WallCubes`) _returnvalue_3))))

(fn `UserConstructionScript`)